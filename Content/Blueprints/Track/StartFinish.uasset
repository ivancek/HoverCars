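; StartFinish is a track actor that counts laps for hover cars and ends a car's race at the lap limit.
; On overlap it runs the parent's handler, casts the actor to TestPawn_BP and increments that pawn's LapsPassed.
; When the count equals NumberOfLaps from the game mode's RaceSettings, it unpossesses the pawn's controller.
; The overlap handler itself makes no check on direction or checkpoints.
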(event EventBeginPlay)

(event Collision|EventActorBeginOverlap
  (params (OtherActor :type Actor%20Object%20Reference))
  (|CallParentFunction OtherActor)
  (bind _astest_pawn_bp (Utilities|Casting|CastToTestPawn_BP OtherActor))
  (bind _output_get (Variables|Default|SetCarThatPassed _astest_pawn_bp))
  (bind _result (Math|Integer|IncrementInt (Variables|/Script/HoverCars.Car|GetLapsPassed _output_get))
    (:%20%20
      (Variables|/Script/HoverCars.Car|SetLapsPassed _astest_pawn_bp _result)
      (bind _ashover_cars_game_mode_bp (Utilities|Casting|CastToHoverCarsGameMode_BP (Game|GetGameMode)))
      (if (== (.numberoflaps (Variables|/Game/Blueprints/Game/HoverCarsGameMode_BP.HoverCarsGameMode_BP_C|GetRaceSettings _ashover_cars_game_mode_bp)) (Variables|/Script/HoverCars.Car|GetLapsPassed (Variables|Default|GetCarThatPassed)))
        (Pawn|UnPossess (Pawn|GetController (Variables|Default|GetCarThatPassed)))))))

(fn ConstructionScript
  (|CallParentFunction))